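; Boat actor that rides along the spline Path of a referenced TracktoMoveOn actor, starting automatically on BeginPlay.
; It snaps to the spline start, then MoveCart plays a timeline at a rate of 1/Duration.
; Timeline alpha maps to distance along the spline, setting location and rotation with a 90-degree yaw offset.
; The ActivateTrigger overlap does nothing, as its FirstPersonCharacter check and MoveCart call are disconnected.
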(event `self.ReceiveBeginPlay`
  (bind _path (`/Game/Blueprint/BP_Track.Path` (`self.TracktoMoveOn`)))
  (bind (_returnvalue_roll _returnvalue_pitch _returnvalue_yaw) (`KismetMathLibrary.BreakRotator` (`SplineComponent.GetRotationAtDistanceAlongSpline` _path 0.0 "World")))
  (`self.K2_SetActorLocationAndRotation` (`SplineComponent.GetLocationAtDistanceAlongSpline` _path 0.0 "World") (`KismetMathLibrary.MakeRotator` _returnvalue_roll _returnvalue_pitch (+ _returnvalue_yaw 90.0)))
  (`self.MoveCart`))

(event `MoveCart`
  (bind _path (`/Game/Blueprint/BP_Track.Path` (`self.TracktoMoveOn`)))
  (bind _returnvalue (`KismetMathLibrary.Lerp` 0.0 (`SplineComponent.GetSplineLength` _path) (`self.Alpha`)))
  (bind (_returnvalue_roll _returnvalue_pitch _returnvalue_yaw) (`KismetMathLibrary.BreakRotator` (`SplineComponent.GetRotationAtDistanceAlongSpline` _path _returnvalue "World")))
  (`TimelineComponent.SetPlayRate` (`self.BoatMovement`) (/ 1.0 (`self.Duration`)))
  (bind (_direction _newtrack_0) (`Timeline|BoatMovement`)
    (:`Update`
      (set `self.Alpha` _newtrack_0)
      (`self.K2_SetActorLocationAndRotation` (`SplineComponent.GetLocationAtDistanceAlongSpline` _path _returnvalue "World") (`KismetMathLibrary.MakeRotator` _returnvalue_roll _returnvalue_pitch (+ _returnvalue_yaw 90.0))))))

(event `self.ActivateTrigger.OnComponentBeginOverlap`
  (params (OverlappedComponent :type "PrimitiveComponent Object Reference") (OtherActor :type "Actor Object Reference") (OtherComp :type "PrimitiveComponent Object Reference") (OtherBodyIndex :type Integer) (bFromSweep :type Boolean) (SweepResult :type "HitResult Structure (by ref)")))

(fn `UserConstructionScript`)