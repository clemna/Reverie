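; BP_Star is an interactable companion that starts following the player when interacted with while exactly three batteries are collected.
; BeginPlay caches the BP_PlayerChar, and Interact starts FollowPlayer.
; FollowPlayer re-triggers itself every 0.2 seconds, using AIMoveTo toward the player at or beyond FollowDistance and toward itself when closer to stay put.
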(event `FollowPlayer`
  (`KismetSystemLibrary.PrintString` "follow")
  (if (>= (`self.GetDistanceTo` (`self.PlayerChar`)) (`self.FollowDistance`))
    (`|AIMoveTo` self (0.0 0.0 0.0) (`self.PlayerChar`)
      (:`then`
        _))
    (else
      (`|AIMoveTo` self (0.0 0.0 0.0) self
        (:`then`
          _))))
  (`KismetSystemLibrary.Delay` 0.2)
  (`self.FollowPlayer`))

(event `self.ReceiveBeginPlay`
  (bind _asbp_player_char (cast `/Game/Blueprint/FirstPersonBP/BP_PlayerChar` (`GameplayStatics.GetPlayerCharacter` 0)))
  (set `self.PlayerChar` _asbp_player_char))

(fn `Interact`
  (params (CollectedBatteries :type Integer) (Rune1 :type Boolean) (Rune2 :type Boolean) (Rune3 :type Boolean) (Keys :type Integer))
  (returns (InteractedObject :type Integer) (RuneCollected :type Boolean))
  (if (not (!= CollectedBatteries 3))
    (`self.FollowPlayer`)
    (`KismetSystemLibrary.PrintString` "follow player"))
  (return 1 false))

(fn `UserConstructionScript`)