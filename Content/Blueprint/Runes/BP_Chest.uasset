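; BP_Chest is an interactable chest among the rune Blueprints that responds only when the player holds a key.
; Its Interact function checks the passed key count, plays a success sound and returns an interacted-object code with no rune collected.
; Event graph events are empty, leaving older logic unwired: an overlap range check and an E-press unlock requiring blue, yellow and green runes.
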(event `self.ReceiveBeginPlay`)

(event `self.ReceiveTick`
  (params (DeltaSeconds :type "Float (single-precision)")))

(event `self.Box.OnComponentBeginOverlap`
  (params (OverlappedComponent :type "PrimitiveComponent Object Reference") (OtherActor :type "Actor Object Reference") (OtherComp :type "PrimitiveComponent Object Reference") (OtherBodyIndex :type Integer) (bFromSweep :type Boolean) (SweepResult :type "HitResult Structure (by ref)")))

(event `self.Box.OnComponentEndOverlap`
  (params (OverlappedComponent :type "PrimitiveComponent Object Reference") (OtherActor :type "Actor Object Reference") (OtherComp :type "PrimitiveComponent Object Reference") (OtherBodyIndex :type Integer)))

(fn `Interact`
  (params (CollectedBatteries :type Integer) (Rune1 :type Boolean) (Rune2 :type Boolean) (Rune3 :type Boolean) (Keys :type Integer))
  (returns (InteractedObject :type Integer) (RuneCollected :type Boolean))
  (if (> Keys 0)
    (`GameplayStatics.PlaySound2D` "/Game/Audio/60443__jobro__tada1.60443__jobro__tada1" 1.0 1.0 0.0 null null)
    (return 2 false)))

(fn `UserConstructionScript`)