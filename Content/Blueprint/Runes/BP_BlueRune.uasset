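; BP_BlueRune is an interactable blue rune that the first-person player activates once to unlock its part of a linked chest.
; An InteractionZone overlap tracks whether the player is in range, and Tick polls the E key while they are.
; On first activation it brightens its point light, then casts LinkedChest to BP_Chest to set its BlueRuneActivated flag and light up the chest's blue light.
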(event `self.ReceiveBeginPlay`
  (set `self.CharController` (`GameplayStatics.GetPlayerController` 0)))

(event `self.ReceiveTick`
  (params (DeltaSeconds :type "Float (single-precision)"))
  (if (and (`self.inRange`) (`PlayerController.WasInputKeyJustPressed` (`self.CharController`) "E"))
    (if (not (`self.activated`))
      (set `self.activated` true)
      (`LightComponent.SetIntensity` (`self.PointLight`) 5000.0)
      (bind _asbp_chest (cast `/Game/Blueprint/Runes/BP_Chest` (`self.LinkedChest`)))
      (set `/Game/Blueprint/Runes/BP_Chest.BlueRuneActivated` true _asbp_chest)
      (`LightComponent.SetIntensity` (`/Game/Blueprint/Runes/BP_Chest.BlueLight` _asbp_chest) 5000.0))))

(event `self.InteractionZone.OnComponentBeginOverlap`
  (params (OverlappedComponent :type "PrimitiveComponent Object Reference") (OtherActor :type "Actor Object Reference") (OtherComp :type "PrimitiveComponent Object Reference") (OtherBodyIndex :type Integer) (bFromSweep :type Boolean) (SweepResult :type "HitResult Structure (by ref)"))
  (cast `/Game/Blueprint/FirstPersonBP/Blueprints/FirstPersonCharacter` OtherActor)
  (set `self.inRange` true))

(event `self.InteractionZone.OnComponentEndOverlap`
  (params (OverlappedComponent :type "PrimitiveComponent Object Reference") (OtherActor :type "Actor Object Reference") (OtherComp :type "PrimitiveComponent Object Reference") (OtherBodyIndex :type Integer))
  (cast `/Game/Blueprint/FirstPersonBP/Blueprints/FirstPersonCharacter` OtherActor)
  (set `self.inRange` false))

(fn `UserConstructionScript`)