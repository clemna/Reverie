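; Star actor that the player activates with E while inside its trigger box, once they have collected at least three batteries.
; Activation happens once, swapping to a stronger material, playing a cheer and starting MoveStar; too few batteries plays a failure sound.
; A timeline, rate-scaled by Duration, drives the star's location and rotation along a referenced track's spline, where it is snapped to the start on BeginPlay.
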(event `self.ReceiveBeginPlay`
  (bind _path (`/Game/Blueprint/BP_Track.Path` (`self.TracktoMoveOn`)))
  (set `self.CharController` (`GameplayStatics.GetPlayerController` 0))
  (`self.K2_SetActorLocationAndRotation` (`SplineComponent.GetLocationAtDistanceAlongSpline` _path 0.0 "World") (`SplineComponent.GetRotationAtDistanceAlongSpline` _path 0.0 "World")))

(event `self.ReceiveTick`
  (params (DeltaSeconds :type "Float (single-precision)"))
  (if (and (`self.inRange`) (`PlayerController.WasInputKeyJustPressed` (`self.CharController`) "E"))
    (if (>= (`/Game/Blueprint/FirstPersonBP/Blueprints/FirstPersonCharacter.BattteriesCollected` (stale `self.Box.OnComponentBeginOverlap` _asfirst_person_character)) 3)
      (if (not (`self.activated`))
        (`PrimitiveComponent.SetMaterial` (`self.Star`) 0 "/Game/Art/Materials/Blockout/m_StarStrong.m_StarStrong")
        (`GameplayStatics.PlaySound2D` "/Game/Sound/428156__higgs01__yay.428156__higgs01__yay" 1.0 1.0 0.0 null null)
        (set `self.activated` true)
        (`self.MoveStar`))
      (else
        (`GameplayStatics.PlaySound2D` "/Game/Sound/519638__marciofao__gear-shif-fail-scratch-1.519638__marciofao__gear-shif-fail-scratch-1" 1.0 1.0 0.0 null null)))))

(event `self.Box.OnComponentBeginOverlap`
  (params (OverlappedComponent :type "PrimitiveComponent Object Reference") (OtherActor :type "Actor Object Reference") (OtherComp :type "PrimitiveComponent Object Reference") (OtherBodyIndex :type Integer) (bFromSweep :type Boolean) (SweepResult :type "HitResult Structure (by ref)"))
  (bind _asfirst_person_character (cast `/Game/Blueprint/FirstPersonBP/Blueprints/FirstPersonCharacter` OtherActor))
  (set `self.inRange` true))

(event `self.Box.OnComponentEndOverlap`
  (params (OverlappedComponent :type "PrimitiveComponent Object Reference") (OtherActor :type "Actor Object Reference") (OtherComp :type "PrimitiveComponent Object Reference") (OtherBodyIndex :type Integer))
  (cast `/Game/Blueprint/FirstPersonBP/Blueprints/FirstPersonCharacter` OtherActor)
  (set `self.inRange` false))

(event `MoveStar`
  (bind _path (`/Game/Blueprint/BP_Track.Path` (`self.TrackToMoveOn`)))
  (bind _returnvalue (`KismetMathLibrary.Lerp` 0.0 (`SplineComponent.GetSplineLength` _path) (`self.Alpha`)))
  (`TimelineComponent.SetPlayRate` (`self.StarMovement`) (/ 1.0 (`self.Duration`)))
  (bind (_direction _newtrack_0) (`Timeline|StarMovement`)
    (:`Update`
      (set `self.Alpha` _newtrack_0)
      (`self.K2_SetActorLocationAndRotation` (`SplineComponent.GetLocationAtDistanceAlongSpline` _path _returnvalue "World") (`SplineComponent.GetRotationAtDistanceAlongSpline` _path _returnvalue "World")))))

(fn `UserConstructionScript`)