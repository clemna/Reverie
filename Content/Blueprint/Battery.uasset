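; Battery is a collectible pickup that adds to the first-person character's collected battery count.
; A Box overlap stores the character and toggles an in-range flag as the player enters and leaves.
; Tick polls the player controller for an E key press while in range, then increments BattteriesCollected on the character and destroys the battery.
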(event `self.ReceiveBeginPlay`
  (set `self.CharController` (`GameplayStatics.GetPlayerController` 0)))

(event `self.ReceiveTick`
  (params (DeltaSeconds :type "Float (single-precision)"))
  (if (and (`self.inRange`) (`PlayerController.WasInputKeyJustPressed` (`self.CharController`) "E"))
    (bind _asfirst_person_character (cast `/Game/Blueprint/FirstPersonBP/Blueprints/FirstPersonCharacter` (stale `self.Box.OnComponentBeginOverlap` _asfirst_person_character)))
    (`/Engine/EditorBlueprintResources/StandardMacros.IncrementInt` (`/Game/Blueprint/FirstPersonBP/Blueprints/FirstPersonCharacter.BattteriesCollected` _asfirst_person_character)
      (:`  `
        (`self.K2_DestroyActor`)))))

(event `self.Box.OnComponentBeginOverlap`
  (params (OverlappedComponent :type "PrimitiveComponent Object Reference") (OtherActor :type "Actor Object Reference") (OtherComp :type "PrimitiveComponent Object Reference") (OtherBodyIndex :type Integer) (bFromSweep :type Boolean) (SweepResult :type "HitResult Structure (by ref)"))
  (bind _asfirst_person_character (cast `/Game/Blueprint/FirstPersonBP/Blueprints/FirstPersonCharacter` OtherActor))
  (set `self.inRange` true))

(event `self.Box.OnComponentEndOverlap`
  (params (OverlappedComponent :type "PrimitiveComponent Object Reference") (OtherActor :type "Actor Object Reference") (OtherComp :type "PrimitiveComponent Object Reference") (OtherBodyIndex :type Integer))
  (cast `/Game/Blueprint/FirstPersonBP/Blueprints/FirstPersonCharacter` OtherActor)
  (set `self.inRange` false))

(fn `UserConstructionScript`)