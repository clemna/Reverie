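; Gate actor that opens by sliding along a spline, keeping its rotation unchanged.
; BeginPlay snaps it to the spline's start.
; The Open_Gate event posts the Wwise gate-open sound, then plays a timeline whose rate is scaled by Duration and whose alpha moves the actor to the spline's end.
; It has no closing logic, and the spline-based yaw calculations are left unconnected.
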(event `self.ReceiveBeginPlay`
  (`self.K2_SetActorLocationAndRotation` (`SplineComponent.GetLocationAtDistanceAlongSpline` (`self.Spline`) 0.0 "World") (`self.K2_GetActorRotation`)))

(event `Open_Gate`
  (bind _spline (`self.Spline`))
  (`AkGameplayStatics.SetOcclusionRefreshInterval` 0.0 self)
  (`AkGameplayStatics.PostEvent` "/Game/Wwise/Events/Play_Gate_Open.Play_Gate_Open" self)
  (`TimelineComponent.SetPlayRate` (`self.Timeline_0`) (/ 0.1 (`self.Duration`)))
  (bind (_direction _newtrack_0) (`Timeline|Timeline_0`)
    (:`Update`
      (set `self.Alpha` _newtrack_0)
      (`self.K2_SetActorLocationAndRotation` (`SplineComponent.GetLocationAtDistanceAlongSpline` _spline (`KismetMathLibrary.Lerp` 0.0 (`SplineComponent.GetSplineLength` _spline) (`self.Alpha`)) "World") (`self.K2_GetActorRotation`)))))

(fn `UserConstructionScript`)