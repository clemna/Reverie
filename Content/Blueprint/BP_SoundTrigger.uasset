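; Trigger actor that starts a Wwise sound when the player character overlaps its Rr component.
; On entry, if not already active, it calls its StopSounds dispatcher, posts its AkEvent and binds Stop_Sound to StopSounds on the referenced StopOnOtherTrigger.
; When that other trigger fires StopSounds, this one posts its stop event and re-arms, so linked triggers can hand audio off to each other.
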(event `self.ReceiveBeginPlay`
  (bind _asbp_player_char (cast `/Game/Blueprint/FirstPersonBP/BP_PlayerChar` (`GameplayStatics.GetPlayerCharacter` 0)))
  (set `self.Player` _asbp_player_char))

(event `self.rr.OnComponentBeginOverlap`
  (params (OverlappedComponent :type "PrimitiveComponent Object Reference") (OtherActor :type "Actor Object Reference") (OtherComp :type "PrimitiveComponent Object Reference") (OtherBodyIndex :type Integer) (bFromSweep :type Boolean) (SweepResult :type "HitResult Structure (by ref)"))
  (if (== OtherActor (`self.Player`))
    (if (not (`self.activated`))
      (`self.StopSounds`)
      (`AkGameplayStatics.PostEvent` (`self.Ak Event`) self)
      (set `self.activated` true)
      (add `self.StopSounds` (`self.StopOnOther Trigger`) (delegate `Stop_Sound`)))))

(event `Stop_Sound`
  (set `self.activated` false)
  (`AkGameplayStatics.PostEvent` (`self.Ak Event_Stop`) self))

(fn `UserConstructionScript`)